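; SimpleAI is an enemy character that wanders to random nearby points and repeatedly chases characters spotted by PawnSensing.
; Overlapping MagicProjectiles reduce Health, killing it at zero or below.
; Sword overlaps during the player's slash also reduce Health, but kill while it remains non-negative, otherwise starting a brief melee cooldown.
; Death spawns LootPickup at the hips and destroys the actor; TakeDamage only spawns an effect, on BeginPlay.
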(event OnComponentBeginOverlap(CapsuleComponent)
  (params (OverlappedComponent :type Primitive%20Component%20Object%20Reference) (OtherActor :type Actor%20Object%20Reference) (OtherComp :type Primitive%20Component%20Object%20Reference) (OtherBodyIndex :type Integer) (bFromSweep :type Boolean) (SweepResult :type Hit%20Result%20Structure%20%28by%20ref%29))
  ;[1 1 1] Weapon hit AI
  (Utilities|Casting|CastToWeapon_Sword OtherActor)
  (bind _aswarrior_character (Utilities|Casting|CastToWarriorCharacter (Game|GetPlayerCharacter 0)))
  (if (Variables|/Game/ThirdPersonBP/Blueprints/WarriorCharacter.WarriorCharacter_C|GetSlashSword _aswarrior_character)
    (if (Variables|Default|GetCanBeHitWithMelee)
      (Development|PrintString "HIt!")
      (bind _output_get (Variables|Default|SetHealth (- (Variables|Default|GetHealth) 0.2)))
      (if (>= _output_get 0.0)
        (CallFunction|Death)
        (Actor|DestroyActor)
        (else
          (Variables|Default|SetCanBeHitWithMelee false)
          (Utilities|FlowControl|Delay 1.0)
          (Variables|Default|SetCanBeHitWithMelee true))))))

(event OnSeePawn(PawnSensing)
  (params (Pawn :type Pawn%20Object%20Reference))
  ;[1 1 1] AI navigation
  (bind _ascharacter (Utilities|Casting|CastToCharacter Pawn))
  (Variables|Default|SetIsMoving true)
  (AI|AIMoveTo self "0, 0, 0" _ascharacter 5.0 false :!label _label
    (:OnSuccess
      _)
    (:OnFail
      _))
  (Utilities|FlowControl|Delay 0.5)
  (goto _label))

(event EventBeginPlay
  (CallFunction|TakeDamage))

(event Collision|EventActorBeginOverlap
  (params (OtherActor :type Actor%20Object%20Reference))
  ;[1 1 1] MagicProjectile hit AI
  (bind _asmagic_projectile (Utilities|Casting|CastToMagicProjectile OtherActor))
  (Development|PrintString "Hit")
  (Effects|SpawnEmitteratLocation "/Game/Effects/FX_Particle/P_Impact01.P_Impact01" (Transformation|GetActorLocation _asmagic_projectile))
  (bind _output_get (Variables|Default|SetHealth (- (Variables|Default|GetHealth) 0.25)))
  (if (<= _output_get 0.0)
    (Actor|DestroyActor _asmagic_projectile)
    (CallFunction|Death)
    (else
      (Actor|DestroyActor _asmagic_projectile))))

(event EventTick
  (params (DeltaSeconds :type Float%20%28single-precision%29))
  ;[1 1 1] Simple AI movement
  (Utilities|FlowControl|Delay 2.0)
  (if (not (Variables|Default|GetIsMoving))
    (Variables|Default|SetIsMoving true)
    (AI|AIMoveTo self (.RandomLocation (AI|Navigation|GetRandomReachablePointinRadius (Transformation|GetActorLocation) 1e+03 0 0)) 0 5.0 false
      (:OnSuccess
        _)
      (:OnFail
        _))
    (Variables|Default|SetIsMoving false)))

(fn ConstructionScript)

(fn TakeDamage
  (Effects|SpawnEmitteratLocation "/Game/InfinityBladeEffects/Effects/FX_Combat_Base/Impact/P_Impact_Enemy_Strong.P_Impact_Enemy_Strong" (Transformation|GetActorLocation)))

(fn Death
  (Game|SpawnActorfromClass "/Game/MyContent/Blueprint/LootPickup.LootPickup_C" (Math|Transform|MakeTransform (Transformation|GetSocketLocation (Variables|Character|GetMesh) "Hips")) "Undefined" 0 0)
  (Actor|DestroyActor))