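; LootPickup is a loot actor that opens a LootBag screen when a MageCharacter or WarriorCharacter overlaps it.
; The Mage uses the actor overlap event and the Warrior the Box overlap, each spawning a particle effect, destroying the pickup, pausing the game and showing the cursor.
; Both paths then converge to fill five ThirdPersonGameMode inventory slots with random integers, after the widget is already on screen.
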(event OnComponentBeginOverlap(Box)
  (params (OverlappedComponent :type Primitive%20Component%20Object%20Reference) (OtherActor :type Actor%20Object%20Reference) (OtherComp :type Primitive%20Component%20Object%20Reference) (OtherBodyIndex :type Integer) (bFromSweep :type Boolean) (SweepResult :type Hit%20Result%20Structure%20%28by%20ref%29))
  ;[1 1 1] Warrior pickup
  (bind _aswarrior_character (Utilities|Casting|CastToWarriorCharacter OtherActor))
  (Effects|SpawnEmitteratLocation "/Game/InfinityBladeEffects/Effects/FX_Treasure/Loot/P_Loot_Pickup.P_Loot_Pickup" (Transformation|GetActorLocation _aswarrior_character))
  (Actor|DestroyActor)
  (bind _returnvalue (UserInterface|CreateWidget "/Game/MyContent/Blueprint/LootBag.LootBag_C"))
  (UserInterface|Viewport|AddtoViewport _returnvalue 0)
  (Game|SetGamePaused true)
  (bind _asplayer_controller (Utilities|Casting|CastToPlayerController (Game|GetPlayerController 0)))
  (Variables|/Script/Engine.PlayerController|SetbShowMouseCursor _asplayer_controller true)
  (bind _asthird_person_game_mode (Utilities|Casting|CastToThirdPersonGameMode (Game|GetGameMode)))
  (Variables|/Game/ThirdPersonBP/Blueprints/ThirdPersonGameMode.ThirdPersonGameMode_C|SetInventorySlot1 _asthird_person_game_mode (Math|Random|RandomIntegerinRange 0 3))
  (Variables|/Game/ThirdPersonBP/Blueprints/ThirdPersonGameMode.ThirdPersonGameMode_C|SetInventorySlot2 _asthird_person_game_mode (Math|Random|RandomIntegerinRange 0 3))
  (Variables|/Game/ThirdPersonBP/Blueprints/ThirdPersonGameMode.ThirdPersonGameMode_C|SetInventorySlot3 _asthird_person_game_mode (Math|Random|RandomIntegerinRange 0 3))
  (Variables|/Game/ThirdPersonBP/Blueprints/ThirdPersonGameMode.ThirdPersonGameMode_C|SetInventorySlot4 _asthird_person_game_mode (Math|Random|RandomIntegerinRange 0 3))
  (Variables|/Game/ThirdPersonBP/Blueprints/ThirdPersonGameMode.ThirdPersonGameMode_C|SetInventorySlot5 _asthird_person_game_mode (Math|Random|RandomIntegerinRange 0 3)))

(event Collision|EventActorBeginOverlap
  (params (OtherActor :type Actor%20Object%20Reference))
  ;[1 1 1] Mage pickup
  (bind _asmage_character (Utilities|Casting|CastToMageCharacter OtherActor))
  (Effects|SpawnEmitteratLocation "/Game/InfinityBladeEffects/Effects/FX_Treasure/Loot/P_Loot_Pickup.P_Loot_Pickup" (Transformation|GetActorLocation _asmage_character))
  (Actor|DestroyActor)
  (bind _returnvalue (UserInterface|CreateWidget "/Game/MyContent/Blueprint/LootBag.LootBag_C"))
  (UserInterface|Viewport|AddtoViewport _returnvalue 0)
  (Game|SetGamePaused true)
  (bind _asplayer_controller (Utilities|Casting|CastToPlayerController (Game|GetPlayerController 0)))
  (Variables|/Script/Engine.PlayerController|SetbShowMouseCursor _asplayer_controller true)
  (bind _asthird_person_game_mode (Utilities|Casting|CastToThirdPersonGameMode (Game|GetGameMode)))
  (Variables|/Game/ThirdPersonBP/Blueprints/ThirdPersonGameMode.ThirdPersonGameMode_C|SetInventorySlot1 _asthird_person_game_mode (Math|Random|RandomIntegerinRange 0 3))
  (Variables|/Game/ThirdPersonBP/Blueprints/ThirdPersonGameMode.ThirdPersonGameMode_C|SetInventorySlot2 _asthird_person_game_mode (Math|Random|RandomIntegerinRange 0 3))
  (Variables|/Game/ThirdPersonBP/Blueprints/ThirdPersonGameMode.ThirdPersonGameMode_C|SetInventorySlot3 _asthird_person_game_mode (Math|Random|RandomIntegerinRange 0 3))
  (Variables|/Game/ThirdPersonBP/Blueprints/ThirdPersonGameMode.ThirdPersonGameMode_C|SetInventorySlot4 _asthird_person_game_mode (Math|Random|RandomIntegerinRange 0 3))
  (Variables|/Game/ThirdPersonBP/Blueprints/ThirdPersonGameMode.ThirdPersonGameMode_C|SetInventorySlot5 _asthird_person_game_mode (Math|Random|RandomIntegerinRange 0 3)))

(fn ConstructionScript)