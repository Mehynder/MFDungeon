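; Key pickup actor that adds itself to the player's inventory when anything overlaps its Box component.
; The overlap casts to ThirdPersonGameMode and checks its eight separate inventory slot variables through a nested branch chain, without filtering the overlapping actor.
; The first empty slot (0) is set to item ID 1 and the actor destroys itself.
; If all slots are occupied, it shows an InventoryFullPopup widget and stays in place.
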(event OnComponentBeginOverlap(Box)
  (params (OverlappedComponent :type Primitive%20Component%20Object%20Reference) (OtherActor :type Actor%20Object%20Reference) (OtherComp :type Primitive%20Component%20Object%20Reference) (OtherBodyIndex :type Integer) (bFromSweep :type Boolean) (SweepResult :type Hit%20Result%20Structure%20%28by%20ref%29))
  (bind _asthird_person_game_mode (Utilities|Casting|CastToThirdPersonGameMode (Game|GetGameMode)))
  (if (== (Variables|/Game/ThirdPersonBP/Blueprints/ThirdPersonGameMode.ThirdPersonGameMode_C|GetInventoryItem1 _asthird_person_game_mode) 0)
    (Variables|/Game/ThirdPersonBP/Blueprints/ThirdPersonGameMode.ThirdPersonGameMode_C|SetInventoryItem1 _asthird_person_game_mode 1)
    (Actor|DestroyActor :!label _label)
    (elif (== (Variables|/Game/ThirdPersonBP/Blueprints/ThirdPersonGameMode.ThirdPersonGameMode_C|GetInventoryItem2 _asthird_person_game_mode) 0)
      (Variables|/Game/ThirdPersonBP/Blueprints/ThirdPersonGameMode.ThirdPersonGameMode_C|SetInventoryItem2 _asthird_person_game_mode 1)
      (goto _label)
      (elif (== (Variables|/Game/ThirdPersonBP/Blueprints/ThirdPersonGameMode.ThirdPersonGameMode_C|GetInventoryItem3 _asthird_person_game_mode) 0)
        (Variables|/Game/ThirdPersonBP/Blueprints/ThirdPersonGameMode.ThirdPersonGameMode_C|SetInventoryItem3 _asthird_person_game_mode 1)
        (goto _label)
        (elif (== (Variables|/Game/ThirdPersonBP/Blueprints/ThirdPersonGameMode.ThirdPersonGameMode_C|GetInventoryItem4 _asthird_person_game_mode) 0)
          (Variables|/Game/ThirdPersonBP/Blueprints/ThirdPersonGameMode.ThirdPersonGameMode_C|SetInventoryItem4 _asthird_person_game_mode 1)
          (goto _label)
          (elif (== (Variables|/Game/ThirdPersonBP/Blueprints/ThirdPersonGameMode.ThirdPersonGameMode_C|GetInventoryItem5 _asthird_person_game_mode) 0)
            (Variables|/Game/ThirdPersonBP/Blueprints/ThirdPersonGameMode.ThirdPersonGameMode_C|SetInventoryItem5 _asthird_person_game_mode 1)
            (goto _label)
            (elif (== (Variables|/Game/ThirdPersonBP/Blueprints/ThirdPersonGameMode.ThirdPersonGameMode_C|GetInventoryItem6 _asthird_person_game_mode) 0)
              (Variables|/Game/ThirdPersonBP/Blueprints/ThirdPersonGameMode.ThirdPersonGameMode_C|SetInventoryItem6 _asthird_person_game_mode 1)
              (goto _label)
              (elif (== (Variables|/Game/ThirdPersonBP/Blueprints/ThirdPersonGameMode.ThirdPersonGameMode_C|GetInventoryItem7 _asthird_person_game_mode) 0)
                (Variables|/Game/ThirdPersonBP/Blueprints/ThirdPersonGameMode.ThirdPersonGameMode_C|SetInventoryItem7 _asthird_person_game_mode 1)
                (goto _label)
                (elif (== (Variables|/Game/ThirdPersonBP/Blueprints/ThirdPersonGameMode.ThirdPersonGameMode_C|GetInventoryItem8 _asthird_person_game_mode) 0)
                  (Variables|/Game/ThirdPersonBP/Blueprints/ThirdPersonGameMode.ThirdPersonGameMode_C|SetInventoryItem8 _asthird_person_game_mode 1)
                  (goto _label)
                  (else
                    (bind _returnvalue (UserInterface|CreateWidget "/Game/MyContent/Blueprint/InventoryFullPopup.InventoryFullPopup_C"))
                    (UserInterface|Viewport|AddtoViewport _returnvalue 0)))))))))))

(event EventBeginPlay)

(event Collision|EventActorBeginOverlap
  (params (OtherActor :type Actor%20Object%20Reference)))

(event EventTick
  (params (DeltaSeconds :type Float%20%28single-precision%29)))

(fn ConstructionScript)